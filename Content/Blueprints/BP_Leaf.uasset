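; BP_Leaf is a possessable physics leaf that the player nudges with force from input axes until it lands.
; Landing triggers on hitting a Landscape, or on near-zero velocity once InitLeaf has enabled ground checks.
; Landed disables input, then after a delay either returns to title or plays a camera transition meant to possess the next leaf.
; BP_PlayerController holds level state and target transforms, and timelines drive the title and restart camera lerps.
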(event OnComponentHit(Leaf)
  (params (HitComponent :type Primitive%20Component%20Object%20Reference) (OtherActor :type Actor%20Object%20Reference) (OtherComp :type Primitive%20Component%20Object%20Reference) (NormalImpulse :type Vector :default "0, 0, 0") (Hit :type Hit%20Result%20Structure%20%28by%20ref%29))
  (if (== (Utilities|GetClass OtherActor) "/Script/Landscape.Landscape")
    (Utilities|FlowControl|DoOnce false
      (:Completed
        (CallFunction|Landed)))))

(event Custom|Landed
  (bind _playercontrollerreference (Variables|References|GetPlayerControllerReference))
  (Input|DisableInput 0)
  (Default|SetNextTransform (Variables|References|GetPlayerControllerReference))
  (Variables|RestartLeaf|SetOnGround true)
  (Utilities|FlowControl|Delay (Variables|Default|GetRestartDelay))
  (if (Variables|/Game/Blueprints/BP_PlayerController.BP_PlayerController_C|GetDone (Variables|References|GetPlayerControllerReference))
    (Variables|/Game/Blueprints/BP_PlayerController.BP_PlayerController_C|SetFinishText _playercontrollerreference "Fin")
    (Default|ReturntoTitle _playercontrollerreference)
    (elif (Variables|/Game/Blueprints/BP_PlayerController.BP_PlayerController_C|GetLevelStarted _playercontrollerreference)
      (Variables|Default|SetCurrentTransform (Transformation|GetWorldTransform (Variables|Default|GetCamera)))
      (Audio|Components|Audio|Play (Variables|Default|GetRestartAnimation))
      (Input|DisableInput (Variables|References|GetPlayerControllerReference)))))

(event Custom|InitLeaf
  (Utilities|FlowControl|Delay 0.5)
  (Physics|SetSimulatePhysics (Variables|Default|GetLeaf) true)
  (Utilities|FlowControl|Delay 1.0)
  (Variables|Default|SetCheckOnGround true)
  (Input|EnableInput 0))

(event EventTick
  (params (DeltaSeconds :type Float%20%28single-precision%29))
  (if (Variables|/Game/Blueprints/BP_PlayerController.BP_PlayerController_C|GetLevelStarted (Variables|References|GetPlayerControllerReference))
    (if (and (Math|Vector|Equal(Vector) (Transformation|GetComponentVelocity (Variables|Default|GetLeaf)) "0, 0, 0" 0.75) (Variables|Default|GetCheckOnGround))
      (Utilities|FlowControl|DoOnce false
        (:Completed
          (CallFunction|Landed))))))

(event EventBeginPlay
  (CallFunction|SetUp))

(event Input|AxisEvents|InputAxisInputLeftRight
  (params (AxisValue :type Float%20%28single-precision%29))
  (Physics|AddForce (Variables|Default|GetLeaf) (Math|Vector|MakeVector 0.0 (* AxisValue (Variables|Default|GetPushForce)) 0.0) "None" false))

(event Input|AxisEvents|InputAxisInputUpDown
  (params (AxisValue :type Float%20%28single-precision%29))
  (Physics|AddForce (Variables|Default|GetLeaf) (Math|Vector|MakeVector (* AxisValue (Variables|Default|GetPushForce)) 0.0 0.0) "None" false))

(fn ConstructionScript
  (bind _leaf (Variables|Default|GetLeaf))
  (Transformation|SetWorldRotation (Variables|Default|GetCamera) (Math|Rotator|FindLookatRotation (Transformation|GetWorldLocation (Variables|Default|GetCamera)) (Transformation|GetWorldLocation _leaf)) false false)
  (Transformation|SetWorldRotation (Variables|Default|GetCamPos) (Math|Rotator|FindLookatRotation (Transformation|GetWorldLocation (Variables|Default|GetCamPos)) (Transformation|GetWorldLocation _leaf)) false false))

(fn SetUp
  (bind _asbp_player_controller (Utilities|Casting|CastToBP_PlayerController (Game|GetPlayerController 0)))
  (bind _output_get (Variables|References|SetPlayerControllerReference _asbp_player_controller))
  (Utilities|SetUpLerpTimeline (Variables|Default|GetTitleAnimation) "/Game/Data/CURVE_Linear.CURVE_Linear" "" (Variables|/Game/Blueprints/BP_PlayerController.BP_PlayerController_C|GetTitleSpeed _output_get))
  (Utilities|SetUpLerpTimeline (Variables|Default|GetRestartAnimation) "/Game/Data/CURVE_Linear.CURVE_Linear" "" (Variables|RestartLeaf|GetAnimationSpeed))
  (Input|DisableInput 0))

(fn SetTitleTransform
  (Transformation|SetWorldTransform (Variables|Default|GetCamera) (Variables|TitleSequence|GetTitleTransform) false false))