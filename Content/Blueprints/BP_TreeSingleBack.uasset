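; Tree actor that manages its leaf actors and hands the player control of one at game start.
; On BeginPlay it gathers BP_Leaf child actors from the Tree component's direct children into a shuffled array.
; It then has the player controller possess the first leaf, placed at its title transform.
; GetNextLeaf steps through the array with a counter, returning each leaf and its CamPos world transform, without a bounds check.
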(event EventBeginPlay
  (CallFunction|FillLeafArray)
  (bind _asbp_player_controller (Utilities|Casting|CastToBP_PlayerController (Game|GetPlayerController 0)))
  (bind _output_get (Variables|References|SetPlayerControllerReference _asbp_player_controller))
  (Pawn|UnPossess _output_get)
  (bind _output_get_2 (Variables|/Game/Blueprints/BP_PlayerController.BP_PlayerController_C|SetPlayerReference _output_get (Utilities|Array|Get(acopy) (Variables|Default|GetTreeLeaves))))
  (Default|SetTitleTransform _output_get_2)
  (Pawn|Possess _output_get _output_get_2))

(fn ConstructionScript)

(fn FillLeafArray
  (for _array_element (Components|GetChildrenComponents (Variables|Default|GetTree) false)
    (bind _leaf_component (Utilities|GetLeafComponent _array_element)
      (:then
        (Utilities|Array|Add (Variables|Default|GetTreeLeaves) _leaf_component))
      (:CastFailed
        (Variables|Debug|SetCastFailed true))))
  (Utilities|Array|Shuffle (Variables|Default|GetTreeLeaves)))

(fn GetNextLeaf
  (bind _output_get (LocalVariables|SetReturnLeaf (Utilities|Array|Get(acopy) (Variables|Default|GetTreeLeaves) (Variables|Default|GetArrayCounter))))
  (Math|Integer|IncrementInt (Variables|Default|GetArrayCounter)
    (:%20%20
      (return _output_get (Transformation|GetWorldTransform (Variables|/Game/Blueprints/BP_Leaf.BP_Leaf_C|GetCamPos _output_get))))))