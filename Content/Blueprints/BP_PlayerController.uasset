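; Player controller for a leaf game that handles the title screen, loading fade and possession of successive leaves from a tree.
; Enter or Space starts play and Z or Escape returns to title or quits, with camera attach/detach and timelines played forward or reversed for the transitions.
; SetNextTransform fetches the next leaf from the tree or marks the game done once all are used, and PossessNextLeaf possesses and initializes that leaf.
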(event Custom|PossessNextLeaf
  (bind _nextleaf (Variables|Default|GetNextLeaf))
  (bind _output_get (Variables|References|SetPlayerReference _nextleaf))
  (Pawn|Possess _output_get)
  (Default|InitLeaf _nextleaf)
  (Input|EnableInput 0))

(event EventBeginPlay
  (Utilities|SetUpLerpTimeline (Variables|Default|GetTitleAnimation) "/Game/Data/CURVE_Linear.CURVE_Linear" "" (Variables|Title|GetTitleSpeed))
  (Utilities|SetUpLerpTimeline (Variables|Default|GetLoadingAnimation) "/Game/Data/CURVE_Linear.CURVE_Linear" "" (Variables|Title|GetLoadSpeed))
  (Input|DisableInput 0)
  (Audio|Components|Audio|Play (Variables|Default|GetLoadingAnimation)))

(event Input|KeyboardEvents|AnyKey
  (params (Key :type Key%20Structure)))

(event Input|KeyboardEvents|Escape
  (params (Key :type Key%20Structure))
  (:Pressed
    (if (Variables|Default|GetDone)
      (Game|QuitGame 0 "Quit")
      (elif (Variables|Title|GetLevelStarted)
        (CallFunction|ReturntoTitle)
        (else
          (Game|QuitGame 0 "Quit"))))))

(event Input|KeyboardEvents|Enter
  (params (Key :type Key%20Structure))
  (:Pressed
    (if (not (Variables|Title|GetLevelStarted))
      (if (not (Variables|Default|GetDone))
        (CallFunction|PlayGame)))))

(event Input|KeyboardEvents|Z
  (params (Key :type Key%20Structure))
  (:Pressed
    (if (Variables|Default|GetDone)
      (Game|QuitGame 0 "Quit")
      (elif (Variables|Title|GetLevelStarted)
        (CallFunction|ReturntoTitle)
        (else
          (Game|QuitGame 0 "Quit"))))))

(event Input|KeyboardEvents|SpaceBar
  (params (Key :type Key%20Structure))
  (:Pressed
    (if (not (Variables|Title|GetLevelStarted))
      (if (not (Variables|Default|GetDone))
        (CallFunction|PlayGame)))))

(fn ConstructionScript)

(fn ReturntoTitle
  (Transformation|DetachFromComponent (Variables|/Game/Blueprints/BP_Leaf.BP_Leaf_C|GetCamera (Variables|References|GetPlayerReference)) "KeepWorld" "KeepWorld" "KeepWorld" true)
  (Utilities|String|Reverse (Variables|Default|GetTitleAnimation))
  (Components|Timeline|ReversefromEnd (Variables|/Game/Blueprints/BP_Leaf.BP_Leaf_C|GetTitleAnimation (Variables|References|GetPlayerReference))))

(fn PlayGame
  (bind _playerreference (Variables|References|GetPlayerReference))
  (Transformation|AttachComponentToComponent (Variables|/Game/Blueprints/BP_Leaf.BP_Leaf_C|GetCamera _playerreference) (Variables|/Game/Blueprints/BP_Leaf.BP_Leaf_C|GetSpringArm _playerreference) "None" "KeepWorld" "KeepWorld" "KeepWorld" true)
  (Audio|Components|Audio|Play (Variables|Default|GetTitleAnimation))
  (Audio|Components|Audio|Play (Variables|/Game/Blueprints/BP_Leaf.BP_Leaf_C|GetTitleAnimation (Variables|References|GetPlayerReference))))

(fn SetNextTransform
  (bind _treereference (Variables|References|GetTreeReference))
  (if (== (Variables|/Game/Blueprints/BP_TreeBase.BP_TreeBase_C|GetArrayCounter _treereference) (Utilities|Array|Length (Variables|/Game/Blueprints/BP_TreeBase.BP_TreeBase_C|GetTreeLeaves _treereference)))
    (Variables|Default|SetDone true)
    (else
      (bind (_leaf _returnvalue) (Default|GetNextLeaf (Variables|References|GetTreeReference)))
      (Variables|Default|SetNextLeaf _leaf)
      (Variables|Default|SetNextTransform _returnvalue))))